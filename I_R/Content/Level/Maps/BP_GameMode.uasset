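; Game mode that tracks the player's score and difficulty and saves a high-score table.
; Each tick while the character is alive adds points multiplied by difficulty, which ChangeDifficulty derives from max walk speed.
; LoadScores rebuilds the saved list, using a DoOnce to insert the score under a hard-coded name before the first lower-or-equal entry or at the end, then saves it.
; BeginPlay plays a start sound.
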(event `AddPoints`
  (params (AddScorePoints :type Integer))
  ;[1 1 1] Add Points
  (set `self.Score` (+ AddScorePoints (`self.Score`))))

(event `LoadScores`
  ;[1 1 1] Saving score
  (bind _returnvalue (`GameplayStatics.LoadGameFromSlot` "BP_Save"))
  (bind _asbp_save (cast `/Game/Level/Maps/Menu/Score/BP_Save` _returnvalue)
    (:`then`
      (for _array_element (`/Game/Level/Maps/Menu/Score/BP_Save.Player Score` _asbp_save)
        (`|ExecutionSequence`
          (:`then_0`
            (if (<= (`.score_9_E3BA201341CB77FF39F6E9A74DA660D5` (break `/Game/Level/Maps/Menu/Score/Player_score` _array_element)) (`self.Score`))
              (`/Engine/EditorBlueprintResources/StandardMacros.DoOnce` false :!label _label
                (:`Completed`
                  (`KismetArrayLibrary.Array_Add` (`self.Temp`) (make `/Game/Level/Maps/Menu/Score/Player_score` "Greg" (`self.Score`)))))))
          (:`then_1`
            (`KismetArrayLibrary.Array_Add` (`self.Temp`) _array_element))))
      (`|ExecutionSequence`
        (:`then_0`
          (goto _label))
        (:`then_1`
          (bind _returnvalue_2 (`GameplayStatics.CreateSaveGameObject` "/Game/Level/Maps/Menu/Score/BP_Save.BP_Save_C" :!label _label_2))
          (bind _asbp_save_2 (cast `/Game/Level/Maps/Menu/Score/BP_Save` _returnvalue_2))
          (set `/Game/Level/Maps/Menu/Score/BP_Save.Player Score` (`self.Temp`) _asbp_save_2)
          (`GameplayStatics.SaveGameToSlot` _asbp_save_2 "BP_Save"))))
    (:`CastFailed`
      (`|ExecutionSequence`
        (:`then_0`
          (goto _label))
        (:`then_1`
          (goto _label_2))))))

(event `self.ReceiveBeginPlay`
  (`GameplayStatics.PlaySound2D` "/Game/Level/Sounds/start_sound.start_sound" 1.0 1.0 0.0 null null))

(event `self.ReceiveTick`
  (params (DeltaSeconds :type "Float (single-precision)"))
  (bind _difficulty_level (`self.difficulty Level`))
  ;[1 1 1] Add score on tick
  (bind _asthird_person_character (cast `/Game/ThirdPersonBP/Blueprints/ThirdPersonCharacter` (`GameplayStatics.GetPlayerPawn` 0)))
  (if (not (`/Game/ThirdPersonBP/Blueprints/ThirdPersonCharacter.IsDead` _asthird_person_character))
    (bind _asbp_game_mode (cast `/Game/Level/Maps/BP_GameMode` (`GameplayStatics.GetGameMode`)))
    (if (>= _difficulty_level 2)
      (if (>= _difficulty_level 3)
        (set `self.Score multi` 4)
        (else
          (set `self.Score multi` 2)))
      (else
        (set `self.Score multi` 1)))
    (`self.AddPoints` _asbp_game_mode (`self.Score multi`))))

(event `Change Difficulty`
  ;[1 1 1] Change difficulty
  (bind _asthird_person_character (cast `/Game/ThirdPersonBP/Blueprints/ThirdPersonCharacter` (`GameplayStatics.GetPlayerPawn` 0)))
  (bind _maxwalkspeed (`CharacterMovementComponent.MaxWalkSpeed` (`Character.CharacterMovement` _asthird_person_character)))
  (if (>= _maxwalkspeed 1800.0)
    (if (>= _maxwalkspeed 2600.0)
      (set `self.difficulty Level` 3)
      (else
        (set `self.difficulty Level` 2)))))

(fn `UserConstructionScript`)