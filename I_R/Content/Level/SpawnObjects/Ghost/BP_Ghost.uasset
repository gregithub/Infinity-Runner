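; BP_Ghost is a spawnable pickup that calls MakeGhost on the ThirdPersonCharacter touching it and awards points through BP_GameMode.
; The Pick_Up_Box overlap plays a sound before the character cast, then applies the effect and points and destroys the actor.
; It also removes itself after a short delay when Destroy_Collision is overlapped, or when the lifespan set on BeginPlay expires.
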(event `self.ReceiveBeginPlay`
  (`self.SetLifeSpan` 20.0))

(event `self.Pick_Up_Box.OnComponentBeginOverlap`
  (params (OverlappedComponent :type "PrimitiveComponent Object Reference") (OtherActor :type "Actor Object Reference") (OtherComp :type "PrimitiveComponent Object Reference") (OtherBodyIndex :type Integer) (bFromSweep :type Boolean) (SweepResult :type "HitResult Structure (by ref)"))
  (`GameplayStatics.PlaySound2D` "/Game/Level/Sounds/pepega_sound.pepega_sound" 1.0 1.0 0.0 null null)
  (bind _asthird_person_character (cast `/Game/ThirdPersonBP/Blueprints/ThirdPersonCharacter` OtherActor))
  (`/Game/ThirdPersonBP/Blueprints/ThirdPersonCharacter.Make ghost` _asthird_person_character)
  (bind _asbp_game_mode (cast `/Game/Level/Maps/BP_GameMode` (`GameplayStatics.GetGameMode`)))
  (`/Game/Level/Maps/BP_GameMode.AddPoints` _asbp_game_mode 200)
  (`self.K2_DestroyActor`))

(event `self.Destroy_Collision.OnComponentBeginOverlap`
  (params (OverlappedComponent :type "PrimitiveComponent Object Reference") (OtherActor :type "Actor Object Reference") (OtherComp :type "PrimitiveComponent Object Reference") (OtherBodyIndex :type Integer) (bFromSweep :type Boolean) (SweepResult :type "HitResult Structure (by ref)"))
  (`KismetSystemLibrary.Delay` 1.0)
  (`self.K2_DestroyActor`))

(fn `UserConstructionScript`)