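; BP_Module_05_ghost is a level module that dresses itself by difficulty, spawns pickups and enemies, and chains to the next module.
; On BeginPlay it sets its tile material from the GameMode's difficulty level, then randomly spawns a ghost one time in four and up to one coin.
; Overlapping its spawn trigger places a random module at its attach point, and overlapping the destroy trigger removes it.
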(event `self.ReceiveBeginPlay`
  ;[1 1 1] Set visual for level
  (bind _asbp_game_mode (cast `/Game/Level/Maps/BP_GameMode` (`GameplayStatics.GetGameMode`)))
  (switch `int` (`/Game/Level/Maps/BP_GameMode.difficulty Level` _asbp_game_mode)
    (:`Default`
      (`PrimitiveComponent.SetMaterial` (`self.StaticMesh`) 0 "/Game/Level/Materials/Tile/M_Tech_Hex_Tile_Pulse_Inst.M_Tech_Hex_Tile_Pulse_Inst" :!label _label))
    (:`1`
      (goto _label))
    (:`2`
      (`PrimitiveComponent.SetMaterial` (`self.StaticMesh`) 0 "/Game/Level/Materials/Tile/M_Tech_Hex_Tile_Pulse_Inst_Level_2.M_Tech_Hex_Tile_Pulse_Inst_Level_2"))
    (:`3`
      (`PrimitiveComponent.SetMaterial` (`self.StaticMesh`) 0 "/Game/Level/Materials/Tile/M_Tech_Hex_Tile_Pulse_Inst_Level_3.M_Tech_Hex_Tile_Pulse_Inst_Level_3")))
  (switch `int` (`KismetMathLibrary.RandomIntegerInRange` 0 3)
    (:`0`
      (`self.Randomly_Spawn_Actors` "/Game/Level/SpawnObjects/Ghost/BP_Ghost.BP_Ghost_C" 1))
    (:`1`
      _)
    (:`2`
      _)
    (:`3`
      _))
  (`self.Randomly_Spawn_Actors` "/Game/Level/SpawnObjects/Coin/BP_Coin.BP_Coin_C" (`KismetMathLibrary.RandomIntegerInRange` 0 1)))

(event `self.Spawn_Next_Room_Collision.OnComponentBeginOverlap`
  (params (OverlappedComponent :type "PrimitiveComponent Object Reference") (OtherActor :type "Actor Object Reference") (OtherComp :type "PrimitiveComponent Object Reference") (OtherBodyIndex :type Integer) (bFromSweep :type Boolean) (SweepResult :type "HitResult Structure (by ref)"))
  (`self.Random_Module_Place` (.location (`SceneComponent.K2_GetComponentToWorld` (`self.AttachPoint`)))))

(event `self.Destroy_Self_Collision.OnComponentBeginOverlap`
  (params (OverlappedComponent :type "PrimitiveComponent Object Reference") (OtherActor :type "Actor Object Reference") (OtherComp :type "PrimitiveComponent Object Reference") (OtherBodyIndex :type Integer) (bFromSweep :type Boolean) (SweepResult :type "HitResult Structure (by ref)"))
  (`self.K2_DestroyActor`))

(fn `UserConstructionScript`)