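; BP_Module_04_wall is a level module that fills itself with a random wall and chains procedurally spawned modules.
; Shortly after BeginPlay, it places one of four wall variants at WallSpawnLocation.
; A one-shot overlap on Spawn_Next_Room_Collision places a random module from five types, itself included, at AttachPoint after a short delay.
; Overlapping Destroy_Self_Collision destroys the module.
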(event `self.ReceiveBeginPlay`
  (bind _wall_spawn_location (`self.Wall_spawn_location`))
  (`KismetSystemLibrary.Delay` 0.5)
  (switch `int` (`KismetMathLibrary.RandomInteger` 4)
    (:`0`
      (`self.PlaceActor` "/Game/Level/SpawnObjects/Obstacles/Wall/BP_Wall_01.BP_Wall_01_C" _wall_spawn_location))
    (:`1`
      (`self.PlaceActor` "/Game/Level/SpawnObjects/Obstacles/Wall/BP_Wall_02.BP_Wall_02_C" _wall_spawn_location))
    (:`2`
      (`self.PlaceActor` "/Game/Level/SpawnObjects/Obstacles/Wall/BP_Wall_03.BP_Wall_03_C" _wall_spawn_location))
    (:`3`
      (`self.PlaceActor` "/Game/Level/SpawnObjects/Obstacles/Wall/BP_Wall_04.BP_Wall_04_C" _wall_spawn_location))))

(event `self.Spawn_Next_Room_Collision.OnComponentBeginOverlap`
  (params (OverlappedComponent :type "PrimitiveComponent Object Reference") (OtherActor :type "Actor Object Reference") (OtherComp :type "PrimitiveComponent Object Reference") (OtherBodyIndex :type Integer) (bFromSweep :type Boolean) (SweepResult :type "HitResult Structure (by ref)"))
  (bind _returnvalue (`SceneComponent.K2_GetComponentLocation` (`self.AttachPoint`)))
  (if (not (`self.Spawn Called`))
    (set `self.Spawn Called` true)
    (`KismetSystemLibrary.Delay` 0.5)
    (switch `int` (`KismetMathLibrary.RandomInteger` 5)
      (:`Default`
        (`self.PlaceModule` "/Game/Level/Modules/BP_Module_00_free.BP_Module_00_free_C" _returnvalue :!label _label))
      (:`0`
        (goto _label))
      (:`1`
        (`self.PlaceModule` "/Game/Level/Modules/BP_Module_01_box.BP_Module_01_box_C" _returnvalue))
      (:`2`
        (`self.PlaceModule` "/Game/Level/Modules/BP_Module_02_pepega.BP_Module_02_pepega_C" _returnvalue))
      (:`3`
        (`self.PlaceModule` "/Game/Level/Modules/BP_Module_03_coin.BP_Module_03_coin_C" _returnvalue))
      (:`4`
        (`self.PlaceModule` "BP_Module_04_wall_C" _returnvalue)))))

(event `self.Destroy_Self_Collision.OnComponentBeginOverlap`
  (params (OverlappedComponent :type "PrimitiveComponent Object Reference") (OtherActor :type "Actor Object Reference") (OtherComp :type "PrimitiveComponent Object Reference") (OtherBodyIndex :type Integer) (bFromSweep :type Boolean) (SweepResult :type "HitResult Structure (by ref)"))
  (`self.K2_DestroyActor`))

(fn `UserConstructionScript`)