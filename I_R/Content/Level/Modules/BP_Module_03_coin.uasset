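; Level module for procedurally chained rooms that scatters coins inside itself.
; Shortly after BeginPlay it randomly spawns two BP_Coin actors.
; An overlap on its spawn trigger places a randomly chosen next module (free, box, pepega or another coin room) at its AttachPoint.
; A separate overlap trigger destroys the module.
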(event `self.ReceiveBeginPlay`
  (`KismetSystemLibrary.Delay` 0.1)
  (`self.Randomly_Spawn_Actors` "/Game/Level/SpawnObjects/Coin/BP_Coin.BP_Coin_C" 2))

(event `self.Spawn_Next_Room_Collision.OnComponentBeginOverlap`
  (params (OverlappedComponent :type "PrimitiveComponent Object Reference") (OtherActor :type "Actor Object Reference") (OtherComp :type "PrimitiveComponent Object Reference") (OtherBodyIndex :type Integer) (bFromSweep :type Boolean) (SweepResult :type "HitResult Structure (by ref)"))
  (bind _returnvalue (`SceneComponent.K2_GetComponentLocation` (`self.AttachPoint`)))
  (switch `int` (`KismetMathLibrary.RandomInteger` 4)
    (:`Default`
      (`self.PlaceModule` "/Game/Level/Modules/BP_Module_00_free.BP_Module_00_free_C" _returnvalue :!label _label))
    (:`0`
      (goto _label))
    (:`1`
      (`self.PlaceModule` "/Game/Level/Modules/BP_Module_01_box.BP_Module_01_box_C" _returnvalue))
    (:`2`
      (`self.PlaceModule` "/Game/Level/Modules/BP_Module_02_pepega.BP_Module_02_pepega_C" _returnvalue))
    (:`3`
      (`self.PlaceModule` "BP_Module_03_coin_C" _returnvalue))))

(event `self.Destroy_Self_Collision.OnComponentBeginOverlap`
  (params (OverlappedComponent :type "PrimitiveComponent Object Reference") (OtherActor :type "Actor Object Reference") (OtherComp :type "PrimitiveComponent Object Reference") (OtherBodyIndex :type Integer) (bFromSweep :type Boolean) (SweepResult :type "HitResult Structure (by ref)"))
  (`self.K2_DestroyActor`))

(fn `UserConstructionScript`)