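; BP_Module_02_pepega is a level module in a chain of procedurally placed rooms that spawns two Pepega actors.
; On BeginPlay it sets its mesh material from the GameMode's difficulty level, then after a short delay scatters the Pepegas.
; Overlapping the next-room trigger places one of five random modules, including itself, at its AttachPoint.
; A separate overlap trigger destroys the module.
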(event `self.ReceiveBeginPlay`
  ;[1 1 1] Set visual for level
  (bind _asbp_game_mode (cast `/Game/Level/Maps/BP_GameMode` (`GameplayStatics.GetGameMode`)))
  (switch `int` (`/Game/Level/Maps/BP_GameMode.difficulty Level` _asbp_game_mode)
    (:`Default`
      (`PrimitiveComponent.SetMaterial` (`self.StaticMesh`) 0 "/Game/Level/Materials/Tile/M_Tech_Hex_Tile_Pulse_Inst_Start.M_Tech_Hex_Tile_Pulse_Inst_Start" :!label _label))
    (:`1`
      (goto _label))
    (:`2`
      (`PrimitiveComponent.SetMaterial` (`self.StaticMesh`) 0 "/Game/Level/Materials/Tile/M_Tech_Hex_Tile_Pulse_Inst_Level_2.M_Tech_Hex_Tile_Pulse_Inst_Level_2"))
    (:`3`
      (`PrimitiveComponent.SetMaterial` (`self.StaticMesh`) 0 "/Game/Level/Materials/Tile/M_Tech_Hex_Tile_Pulse_Inst_Level_3.M_Tech_Hex_Tile_Pulse_Inst_Level_3")))
  (`KismetSystemLibrary.Delay` 0.5)
  (`self.Randomly_Spawn_Actors` "/Game/Level/SpawnObjects/Pepega/BP_Pepega.BP_Pepega_C" 2))

(event `self.Spawn_Next_Room_Collision.OnComponentBeginOverlap`
  (params (OverlappedComponent :type "PrimitiveComponent Object Reference") (OtherActor :type "Actor Object Reference") (OtherComp :type "PrimitiveComponent Object Reference") (OtherBodyIndex :type Integer) (bFromSweep :type Boolean) (SweepResult :type "HitResult Structure (by ref)"))
  (bind _returnvalue (`SceneComponent.K2_GetComponentLocation` (`self.AttachPoint`)))
  (`KismetSystemLibrary.Delay` 0.5)
  (switch `int` (`KismetMathLibrary.RandomIntegerInRange` 0 4)
    (:`Default`
      (`self.PlaceModule` "/Game/Level/Modules/BP_Module_00_free.BP_Module_00_free_C" _returnvalue :!label _label_2))
    (:`0`
      (goto _label_2))
    (:`1`
      (`self.PlaceModule` "/Game/Level/Modules/BP_Module_01_box.BP_Module_01_box_C" _returnvalue))
    (:`2`
      (`self.PlaceModule` "BP_Module_02_pepega_C" _returnvalue))
    (:`3`
      (`self.PlaceModule` "/Game/Level/Modules/BP_Module_03_coin.BP_Module_03_coin_C" _returnvalue))
    (:`4`
      (`self.PlaceModule` "/Game/Level/Modules/BP_Module_04_wall.BP_Module_04_wall_C" _returnvalue))))

(event `self.Destroy_Self_Collision.OnComponentBeginOverlap`
  (params (OverlappedComponent :type "PrimitiveComponent Object Reference") (OtherActor :type "Actor Object Reference") (OtherComp :type "PrimitiveComponent Object Reference") (OtherBodyIndex :type Integer) (bFromSweep :type Boolean) (SweepResult :type "HitResult Structure (by ref)"))
  (`self.K2_DestroyActor`))

(fn `UserConstructionScript`)